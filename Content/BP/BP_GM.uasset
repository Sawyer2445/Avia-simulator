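; BP_GM is a game mode style Blueprint that owns the HUD and handles the end of a mission.
; On BeginPlay it creates WBP_HUD and adds it to the viewport.
; CompleteMission collapses the HUD, shows WBP_GameOver with its Success flag set from the Succes input, then opens the MainMenu level after a short delay.
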(event `self.ReceiveBeginPlay`
  (bind _returnvalue (`|CreateWidget` "/Game/BP/WBP_HUD.WBP_HUD_C"))
  (`UserWidget.AddToViewport` _returnvalue 0))

(event `self.CompleteMission`
  (params (bSucces :type Boolean))
  ;[1 1 1] Скрываем интерфейс и создаём надпись  на экране
  (`Widget.SetVisibility` (stale `self.ReceiveBeginPlay` _returnvalue) "Collapsed")
  (bind _returnvalue (`|CreateWidget` "/Game/BP/WBP_GameOver.WBP_GameOver_C"))
  ;[1 1 1] Выбор типа надписи
  (if bSucces
    (set `/Game/BP/WBP_GameOver.bSuccess` true _returnvalue)
    (else
      (set `/Game/BP/WBP_GameOver.bSuccess` false _returnvalue)))
  ;[1 1 1] Отображать 5 секунд
  (`UserWidget.AddToViewport` _returnvalue 0)
  (`KismetSystemLibrary.Delay` 5.0)
  ;[1 1 1] Открытие главного меню
  (`GameplayStatics.OpenLevel` "MainMenu"))

(fn `UserConstructionScript`)